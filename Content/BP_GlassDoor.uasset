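; BP_GlassDoor is a door actor that prompts the first-person character to press F when it enters the box trigger.
; Pressing F plays a 2D sound, then after a short delay hides the Scene component without its children, prints a debug string and teleports the actor to a fixed location.
; The F handler has no overlap check, and the end-overlap event only casts.
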(event OnComponentBeginOverlap(Box)
  (params (OverlappedComponent :type Primitive%20Component%20Object%20Reference) (OtherActor :type Actor%20Object%20Reference) (OtherComp :type Primitive%20Component%20Object%20Reference) (OtherBodyIndex :type Integer) (bFromSweep :type Boolean) (SweepResult :type Hit%20Result%20Structure%20%28by%20ref%29))
  (Utilities|Casting|CastToBP_FirstPersonCharacter OtherActor)
  (Development|PrintString "Press F to open the door"))

(event OnComponentEndOverlap(Box)
  (params (OverlappedComponent :type Primitive%20Component%20Object%20Reference) (OtherActor :type Actor%20Object%20Reference) (OtherComp :type Primitive%20Component%20Object%20Reference) (OtherBodyIndex :type Integer))
  (Utilities|Casting|CastToBP_FirstPersonCharacter OtherActor))

(event Collision|EventActorBeginOverlap
  (params (OtherActor :type Actor%20Object%20Reference)))

(event EventTick
  (params (DeltaSeconds :type Float%20%28single-precision%29)))

(event Input|KeyboardEvents|F
  (params (Key :type Key%20Structure :default "None"))
  (:Pressed
    (Audio|PlaySound2D "/Game/im-a-gnome-meme-sound-effect-woo.im-a-gnome-meme-sound-effect-woo" 1.0 1.0 0.0 0 0)
    (Utilities|FlowControl|Delay 0.5)
    (Rendering|SetVisibility (Variables|Default|Getscene) false false)
    (Development|PrintString "OOOO")
    (Transformation|SetActorLocation (Math|Vector|MakeVector 0.0 0.0 1e+02) false false)))

(fn ConstructionScript)