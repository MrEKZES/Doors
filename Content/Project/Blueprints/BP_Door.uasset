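; Door actor that swings open when the required number of pedestals is active.
; The OpenTheDoor event checks that ActivePedestalCount equals ActivePedestalNeeded, then plays a timeline that lerps the Box component's relative rotation from start to end.
; BeginPlay caches a single BP_Pedestal reference, which this graph never uses, and the active count is not updated here.
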(event Custom|OpenTheDoor
  (if (== (Variables|Int|GetActivePedestalCount) (Variables|Int|GetActivePedestalNeeded))
    (bind _opendoor (Timeline|OpenDoor Play)
      (:Update
        (Transformation|SetRelativeRotation (Variables|Default|GetBox) (Math|Rotator|Lerp(Rotator) (Variables|Rotation|GetStartRotation) (Variables|Rotation|GetEndRotation) _opendoor) false false)))))

(event EventBeginPlay
  (bind _returnvalue (Actor|GetActorOfClass "/Game/Project/Blueprints/BP_Pedestal.BP_Pedestal_C"))
  (Variables|Default|SetBP_Pedestal _returnvalue))

(event Collision|EventActorBeginOverlap
  (params (OtherActor :type Actor%20Object%20Reference)))

(event EventTick
  (params (DeltaSeconds :type Float%20%28single-precision%29)))

(fn ConstructionScript)