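; BP_Pedestal is a pressure-pedestal trigger that helps open the BP_Door sharing its ID, found among all doors on BeginPlay.
; Box overlaps count keys and toggle IsBusy, hiding the text while occupied, adjusting the door's ActivePedestalCount and calling OpenTheDoor.
; Overlap ID checks reuse the BeginPlay loop's element rather than BPDoor.
; KeysCount decrements only on the releasing path, so exits with multiple keys leave it unchanged.
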(event OnComponentBeginOverlap(Box)
  (params (OverlappedComponent :type Primitive%20Component%20Object%20Reference) (OtherActor :type Actor%20Object%20Reference) (OtherComp :type Primitive%20Component%20Object%20Reference) (OtherBodyIndex :type Integer) (bFromSweep :type Boolean) (SweepResult :type Hit%20Result%20Structure%20%28by%20ref%29))
  (bind _bp_door (Variables|Default|GetBP_Door))
  (Math|Integer|IncrementInt (Variables|Default|GetKeysCount)
    (:%20%20
      (if (not (Variables|Default|GetbIsBusy))
        (Variables|Default|SetbIsBusy true)
        (Rendering|SetVisibility (Variables|Default|GetTextRender) false false)
        (if (== (Variables|/Game/Project/Blueprints/BP_Door.BP_Door_C|GetID (stale EventBeginPlay _array_element)) (Variables|Default|GetID))
          (Math|Integer|IncrementInt (Variables|/Game/Project/Blueprints/BP_Door.BP_Door_C|GetActivePedestalCount _bp_door)
            (:%20%20
              (Default|OpentheDoor _bp_door))))))))

(event OnComponentEndOverlap(Box)
  (params (OverlappedComponent :type Primitive%20Component%20Object%20Reference) (OtherActor :type Actor%20Object%20Reference) (OtherComp :type Primitive%20Component%20Object%20Reference) (OtherBodyIndex :type Integer))
  (bind _bp_door (Variables|Default|GetBP_Door))
  (if (not (> (Variables|Default|GetKeysCount) 1))
    (if (Variables|Default|GetbIsBusy)
      (Variables|Default|SetbIsBusy false)
      (Rendering|SetVisibility (Variables|Default|GetTextRender) true false)
      (if (== (Variables|/Game/Project/Blueprints/BP_Door.BP_Door_C|GetID (stale EventBeginPlay _array_element)) (Variables|Default|GetID))
        (Math|Integer|DecrementInt (Variables|/Game/Project/Blueprints/BP_Door.BP_Door_C|GetActivePedestalCount _bp_door)
          (:%20%20
            (Default|OpentheDoor _bp_door)
            (Math|Integer|DecrementInt (Variables|Default|GetKeysCount))))))))

(event EventBeginPlay
  (bind _outactors (Actor|GetAllActorsOfClass "/Game/Project/Blueprints/BP_Door.BP_Door_C"))
  (for _array_element _outactors
    (if (== (Variables|/Game/Project/Blueprints/BP_Door.BP_Door_C|GetID _array_element) (Variables|Default|GetID))
      (Variables|Default|SetBP_Door _array_element))))

(fn ConstructionScript)